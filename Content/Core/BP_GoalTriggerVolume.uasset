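; Goal trigger volume for a Pong game that awards a point when a BP_Ball overlaps it.
; The ball first takes the owning paddle's color and a new force direction, if that paddle is valid, because game over destroys the ball.
; It then adds score to TeamToScore through GM_Pong and plays a 2D score sound.
; The construction script sizes the box collision from BoxExtent.
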(event `self.ReceiveActorBeginOverlap`
  (params (OtherActor :type "Actor Object Reference"))
  (bind _owningpaddle (`self.OwningPaddle`))
  (bind _asbp_ball (cast `/Game/Core/BP_Ball` OtherActor))
  (`|ExecutionSequence`
    (:`then_0`
      (`/Engine/EditorBlueprintResources/StandardMacros.IsValid` _owningpaddle
        (:`Is Valid`
          (`PongBall.UpdateColor` _asbp_ball (`PongPaddle.Color` _owningpaddle))
          (`PongBall.UpdateForceDirection` _asbp_ball (`self.NewDirection`)))))
    (:`then_1`
      (`/Game/Core/GM_Pong.AddScoreToPlayer` (cast `/Game/Core/GM_Pong` (`GameplayStatics.GetGameMode`) :!pure true) (`self.TeamToScore`)))
    (:`then_2`
      (`GameplayStatics.PlaySound2D` "/Game/SFX/SFX_PongBall_Score.SFX_PongBall_Score" 1.0 1.0 0.0 null null))))

(fn `UserConstructionScript`
  (`BoxComponent.SetBoxExtent` (`self.BoxCollision`) (`self.BoxExtent`) true))