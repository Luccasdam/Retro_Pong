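; Player controller for a Pong game that lets two local players share one controller, each moving their own paddle.
; On BeginPlay it finds all BP_Paddle actors, slots them into an array by their Player value and adds the gameplay Enhanced Input mapping context.
; Per-player up and down actions send movement input to the matching paddle, while the Start action asks GM_Pong to begin play.
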(event `self.ReceiveBeginPlay`
  (bind _outactors (`GameplayStatics.GetAllActorsOfClass` "/Game/Core/BP_Paddle.BP_Paddle_C"))
  (set `self.Paddles` _outactors)
  (for _array_element _outactors
    (switch `EPlayer` (`PongPaddle.Player` _array_element)
      (:`One`
        (`KismetArrayLibrary.Array_Set` (`self.Paddles`) 0 _array_element))
      (:`Two`
        (`KismetArrayLibrary.Array_Set` (`self.Paddles`) 1 _array_element))))
  (`EnhancedInputSubsystemInterface.AddMappingContext` (pcsubsystem `EnhancedInputLocalPlayerSubsystem` self) "/Game/Inputs/IMC_Gameplay.IMC_Gameplay" 0 (struct)))

(event `EnhancedInput|/Game/Inputs/IA_MoveUp_P1`
  (params (ActionValue :type Boolean) (ElapsedSeconds :type "Float (double-precision)") (TriggeredSeconds :type "Float (double-precision)") (InputAction :type "InputAction Object Reference" :default "/Game/Inputs/IA_MoveUp_P1.IA_MoveUp_P1"))
  (:`Triggered`
    (`PongPaddle.AddPaddleMovementInput` (`|GetArrayItem` (`self.Paddles`)) "Up")))

(event `EnhancedInput|/Game/Inputs/IA_MoveUp_P2`
  (params (ActionValue :type Boolean) (ElapsedSeconds :type "Float (double-precision)") (TriggeredSeconds :type "Float (double-precision)") (InputAction :type "InputAction Object Reference" :default "/Game/Inputs/IA_MoveUp_P2.IA_MoveUp_P2"))
  (:`Triggered`
    (`PongPaddle.AddPaddleMovementInput` (`|GetArrayItem` (`self.Paddles`) 1) "Up")))

(event `EnhancedInput|/Game/Inputs/IA_MoveDown_P2`
  (params (ActionValue :type Boolean) (ElapsedSeconds :type "Float (double-precision)") (TriggeredSeconds :type "Float (double-precision)") (InputAction :type "InputAction Object Reference" :default "/Game/Inputs/IA_MoveDown_P2.IA_MoveDown_P2"))
  (:`Triggered`
    (`PongPaddle.AddPaddleMovementInput` (`|GetArrayItem` (`self.Paddles`) 1) "Down")))

(event `EnhancedInput|/Game/Inputs/IA_MoveDown_P1`
  (params (ActionValue :type Boolean) (ElapsedSeconds :type "Float (double-precision)") (TriggeredSeconds :type "Float (double-precision)") (InputAction :type "InputAction Object Reference" :default "/Game/Inputs/IA_MoveDown_P1.IA_MoveDown_P1"))
  (:`Triggered`
    (`PongPaddle.AddPaddleMovementInput` (`|GetArrayItem` (`self.Paddles`)) "Down")))

(event `EnhancedInput|/Game/Inputs/IA_Start`
  (params (ActionValue :type Boolean) (ElapsedSeconds :type "Float (double-precision)") (TriggeredSeconds :type "Float (double-precision)") (InputAction :type "InputAction Object Reference" :default "/Game/Inputs/IA_Start.IA_Start"))
  (:`Triggered`
    (bind _asgm_pong (cast `/Game/Core/GM_Pong` (`GameplayStatics.GetGameMode`)))
    (`/Game/Core/GM_Pong.RequestPlay` _asgm_pong)))

(fn `UserConstructionScript`)