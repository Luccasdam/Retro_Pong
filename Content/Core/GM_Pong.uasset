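; Game mode for Pong that drives match flow and owns the ball's lifecycle.
; It listens for state changes on GS_Pong, spawning the ball and resetting the game on Init, then resetting, launching or destroying it for Waiting, Playing and Game Over.
; RequestPlay advances the state from Welcome, Waiting or Game Over.
; AddScoreToPlayer ends the match at the win condition, otherwise returns to Waiting.
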(event `self.ReceiveBeginPlay`
  (bind _asgs_pong (cast `/Game/Core/GS_Pong` (`GameplayStatics.GetGameState`)))
  (add `/Game/Core/GS_Pong.OnGameStateChanged` _asgs_pong (delegate `OnGameStateChanged_Event`))
  (`self.HandleGameStateChanged` (`/Game/Core/GS_Pong.CurrentGameState` _asgs_pong)))

(event `OnGameStateChanged_Event`
  (params (NewGameState :type "/Game/Statics/EGameState Enum" :default "NewEnumerator0"))
  (`self.HandleGameStateChanged` NewGameState))

(fn `AddScoreToPlayer`
  (params (InPlayer :type "EPlayer Enum" :default "One"))
  (bind _asgs_pong (cast `/Game/Core/GS_Pong` (`GameplayStatics.GetGameState`)))
  (bind _newscore (`/Game/Core/GS_Pong.AddScoreToPlayer` _asgs_pong InPlayer))
  (if (>= _newscore (`/Game/Core/GS_Pong.WinCondition` _asgs_pong))
    (`/Game/Core/GS_Pong.UpdateGameState` _asgs_pong "NewEnumerator3")
    (else
      (`/Game/Core/GS_Pong.UpdateGameState` _asgs_pong "NewEnumerator1"))))

(fn `DestroyTheBall`
  (bind _pongball (`self.PongBall`))
  (`/Engine/EditorBlueprintResources/StandardMacros.IsValid` _pongball
    (:`Is Valid`
      (`self.K2_DestroyActor` _pongball))))

(fn `HandleGameStateChanged`
  (params (InGameState :type "/Game/Statics/EGameState Enum" :default "NewEnumerator0"))
  (switch `/Game/Statics/EGameState` InGameState
    (:`NewEnumerator4`
      (`self.SpawnTheBall`)
      (bind _asgs_pong (cast `/Game/Core/GS_Pong` (`GameplayStatics.GetGameState`)))
      (`/Game/Core/GS_Pong.ResetGame` _asgs_pong)
      (`/Game/Core/GS_Pong.UpdateGameState` _asgs_pong "NewEnumerator1"))
    (:`NewEnumerator1`
      (`self.ResetTheBall`))
    (:`NewEnumerator2`
      (`self.LaunchTheBall`))
    (:`NewEnumerator3`
      (`self.DestroyTheBall`))))

(fn `LaunchTheBall`
  (bind _pongball (`self.PongBall`))
  (`/Engine/EditorBlueprintResources/StandardMacros.IsValid` _pongball
    (:`Is Valid`
      (`PongBall.Launch` _pongball))))

(fn `RequestPlay`
  (bind _asgs_pong (cast `/Game/Core/GS_Pong` (`GameplayStatics.GetGameState`)))
  (switch `/Game/Statics/EGameState` (`/Game/Core/GS_Pong.CurrentGameState` _asgs_pong)
    (:`NewEnumerator0`
      (`/Game/Core/GS_Pong.UpdateGameState` _asgs_pong "NewEnumerator4"))
    (:`NewEnumerator1`
      (`/Game/Core/GS_Pong.UpdateGameState` _asgs_pong "NewEnumerator2"))
    (:`NewEnumerator3`
      (`/Game/Core/GS_Pong.UpdateGameState` _asgs_pong "NewEnumerator4"))))

(fn `ResetTheBall`
  (bind _pongball (`self.PongBall`))
  (`/Engine/EditorBlueprintResources/StandardMacros.IsValid` _pongball
    (:`Is Valid`
      (`PongBall.Reset` _pongball))))

(fn `SpawnTheBall`
  (bind _returnvalue (`|SpawnActorFromClass` "/Game/Core/BP_Ball.BP_Ball_C" (`KismetMathLibrary.MakeTransform` (0.0 0.0 0.0)) "Undefined" "MultiplyWithRoot" self null))
  (bind _output_get (set `self.PongBall` _returnvalue))
  (`KismetSystemLibrary.PrintString` (`KismetStringLibrary.Concat_StrStr` (`KismetSystemLibrary.GetDisplayName` _output_get) " Spawned")))

(fn `UserConstructionScript`)